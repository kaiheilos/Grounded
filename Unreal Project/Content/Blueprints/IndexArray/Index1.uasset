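; Input-driven actor that gives the player a rock spawning menu and tuning of free building placement distance.
; On BeginPlay it enables input and creates a collapsed UI_RockMenu, storing it only if none already exists.
; The Equals key flip-flops menu visibility, cursor and input mode, while P calls the menu's SpawnItem.
; Bracket keys step FreeBuildingPlacementDistance down or up on the SurvivalPlayerCharacter's BuildingPlacementComponent.
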(event EventBeginPlay
  (Input|EnableInput (Game|GetPlayerController 0))
  (bind _foundwidgets (Widget|GetAllWidgetsOfClass "/Game/UI/UI_RockMenu.UI_RockMenu_C" false))
  (if (== (Utilities|Array|Length _foundwidgets) 0)
    (bind _returnvalue (UserInterface|CreateWidget "/Game/UI/UI_RockMenu.UI_RockMenu_C" (Game|GetPlayerController 0)))
    (bind _output_get (Variables|Default|SetRockMenu _returnvalue))
    (UserInterface|Viewport|AddtoViewport _returnvalue 0)
    (Widget|SetVisibility _output_get "Collapsed")))

(event Input|KeyboardEvents|Equals
  (params (Key :type Key%20Structure :default "None"))
  (bind _returnvalue (Game|GetPlayerController 0))
  (:Pressed
    (bind _rockmenu (Variables|Default|GetRockMenu)
      (:then
        (Utilities|FlowControl|FlipFlop
          (:A
            (Widget|SetVisibility _rockmenu "Visible")
            (Variables|/Script/Engine.PlayerController|SetbShowMouseCursor _returnvalue true)
            (Input|SetInputModeGameandUI _returnvalue _rockmenu "LockAlways" false))
          (:B
            (Widget|SetVisibility _rockmenu "Collapsed")
            (Variables|/Script/Engine.PlayerController|SetbShowMouseCursor _returnvalue false)
            (Input|SetInputModeGameOnly _returnvalue))))
      (:else))))

(event Input|KeyboardEvents|P
  (params (Key :type Key%20Structure :default "None"))
  (:Pressed
    (Default|SpawnItem (Variables|Default|GetRockMenu))))

(event Input|KeyboardEvents|LeftBracket
  (params (Key :type Key%20Structure :default "None"))
  (bind _returnvalue (Game|Player|GetPlayerPawn 0))
  (bind _assurvival_player_character (Utilities|Casting|CastToSurvivalPlayerCharacter _returnvalue))
  (bind _buildingplacementcomponent (Variables|/Script/Maine.SurvivalPlayerCharacter|GetBuildingPlacementComponent _assurvival_player_character))
  (:Pressed
    (Variables|/Script/Maine.BuildingPlacementComponent|SetFreeBuildingPlacementDistance _buildingplacementcomponent (- (Variables|/Script/Maine.BuildingPlacementComponent|GetFreeBuildingPlacementDistance _buildingplacementcomponent) 1e+02))))

(event Input|KeyboardEvents|RightBracket
  (params (Key :type Key%20Structure :default "None"))
  (bind _returnvalue (Game|Player|GetPlayerPawn 0))
  (bind _assurvival_player_character (Utilities|Casting|CastToSurvivalPlayerCharacter _returnvalue))
  (bind _buildingplacementcomponent (Variables|/Script/Maine.SurvivalPlayerCharacter|GetBuildingPlacementComponent _assurvival_player_character))
  (:Pressed
    (Variables|/Script/Maine.BuildingPlacementComponent|SetFreeBuildingPlacementDistance _buildingplacementcomponent (+ (Variables|/Script/Maine.BuildingPlacementComponent|GetFreeBuildingPlacementDistance _buildingplacementcomponent) 1e+02))))

(fn ConstructionScript)