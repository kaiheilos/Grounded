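; BP_MenuActor is a world-placed actor that provides a toggleable rock menu (UI_RockMenu) for the local player.
; On BeginPlay it enables input and, only if no UI_RockMenu exists yet, creates one, adds it to the viewport collapsed and stores it.
; The Divide key flips the stored menu between visible and collapsed, showing or hiding the mouse cursor to match.
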(event EventBeginPlay
  (Input|EnableInput (Game|GetPlayerController 0))
  (bind _foundwidgets (Widget|GetAllWidgetsOfClass "/Game/UI/UI_RockMenu.UI_RockMenu_C" false))
  (if (== (Utilities|Array|Length _foundwidgets) 0)
    (bind _returnvalue (UserInterface|CreateWidget "/Game/UI/UI_RockMenu.UI_RockMenu_C" (Game|GetPlayerController 0)))
    (bind _output_get (Variables|Default|SetRockMenu _returnvalue))
    (UserInterface|Viewport|AddtoViewport _returnvalue 0)
    (Widget|SetVisibility _output_get "Collapsed")))

(event Input|KeyboardEvents|Divide
  (params (Key :type Key%20Structure :default "None"))
  (bind _returnvalue (Game|GetPlayerController 0))
  (:Pressed
    (bind _rockmenu (Variables|Default|GetRockMenu)
      (:then
        (Utilities|FlowControl|FlipFlop
          (:A
            (Widget|SetVisibility _rockmenu "Visible")
            (Variables|/Script/Engine.PlayerController|SetbShowMouseCursor _returnvalue true))
          (:B
            (Widget|SetVisibility _rockmenu "Collapsed")
            (Variables|/Script/Engine.PlayerController|SetbShowMouseCursor _returnvalue false))))
      (:else))))

(fn ConstructionScript)